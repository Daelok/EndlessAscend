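; Grappling hook component that fires a hook and pulls its owning Character toward where it hits.
; FireGrapple spawns a moving hook actor plus a cable actor linking owner to hook, binding the hook's hit and destroyed events.
; A hit lowers friction and gravity and adds an impulse-like velocity boost, then Tick applies pulling force until the owner gets close.
; Destroying the hook, on arrival or cancel, removes the cable and resets state and movement settings.
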(event `self.ReceiveTick`
  (params (DeltaSeconds :type "Float (single-precision)"))
  (switch `/Game/Blueprints/E_GrappleState` (`self.GrappleState`)
    (:`NewEnumerator2`
      (bind _ascharacter (cast `Character` (`self.GetOwner`)))
      (`CharacterMovementComponent.AddForce` (`Character.CharacterMovement` _ascharacter) (* (`self.ToGrappleHook`) 100000.0))
      (if (< (`KismetMathLibrary.Vector_Distance` (`Actor.K2_GetActorLocation` (`self.GrappleHook`)) (`Actor.K2_GetActorLocation` (`self.GetOwner`))) 500.0)
        (`Actor.K2_DestroyActor` (`self.GrappleHook`))))))

(fn `CancelGrapple`
  (bind _grapplehook (`self.GrappleHook`)
    (:`then`
      (`Actor.K2_DestroyActor` _grapplehook))
    (:`else`)))

(fn `FireGrapple`
  (params (TargetLocation :type "Vector Structure") (LocalOffset :type "Vector Structure"))
  (locals (FireDirection :type "Vector Structure" :default (0.0 0.0 0.0)))
  (bind _returnvalue (`KismetMathLibrary.MakeRotFromX` (`local.FireDirection`)))
  (if (not (`self.IsInUse?`))
    (set `self.GrappleState` "NewEnumerator1")
    (set `local.FireDirection` (`KismetMathLibrary.Normal` (- (`local.TargetLocation`) (`self.GrappleStartLocation` (`local.LocalOffset`)))))
    (bind _returnvalue_2 (`|SpawnActorFromClass` "/Game/Blueprints/BP_GrappleHook.BP_GrappleHook_C" (`KismetMathLibrary.MakeTransform` (`self.GrappleStartLocation` (`local.LocalOffset`)) _returnvalue) "Undefined" "OverrideRootScale" null (* (`local.FireDirection`) (`self.Speed`)) 5000.0 null))
    (bind _output_get (set `self.GrappleHook` _returnvalue_2))
    (add `Actor.OnActorHit` _output_get (`|CreateDelegate` :!event `OnGrappleHit`))
    (add `Actor.OnDestroyed` (`self.GrappleHook`) (`|CreateDelegate` :!event `On Grapple Hook Destroyed`))
    (bind _returnvalue_3 (`|SpawnActorFromClass` "/Game/Blueprints/BP_GrappleCable.BP_GrappleCable_C" (`KismetMathLibrary.MakeTransform` (`self.GrappleStartLocation` (`local.LocalOffset`)) _returnvalue) "Undefined" "OverrideRootScale" null null))
    (bind _output_get_2 (set `self.GrappleCable` _returnvalue_3))
    (`Actor.K2_AttachToActor` _output_get_2 (`self.GetOwner`) "None" "KeepWorld" "KeepWorld" "KeepWorld" true)
    (`CableComponent.SetAttachEndTo` (`CableActor.CableComponent` (`self.GrappleCable`)) (`self.GrappleHook`) "None" "None")
    (set `CableComponent.EndLocation` (0.0 0.0 0.0) (`CableActor.CableComponent` (`self.GrappleCable`)))))

(fn `IsInUse?`
  (returns (Result :type Boolean))
  (return (select `/Game/Blueprints/E_GrappleState` (`self.GrappleState`) :`NewEnumerator1` true :`NewEnumerator2` true)))

(fn `On Grapple Hook Destroyed`
  (params (DestroyedActor :type "Actor Object Reference"))
  (set `self.GrappleHook` null)
  (set `self.GrappleState` "NewEnumerator0")
  (`|ExecutionSequence`
    (:`then_0`
      (bind _grapplecable (`self.GrappleCable`)
        (:`then`
          (`Actor.K2_DestroyActor` _grapplecable)
          (set `self.GrappleCable` null))
        (:`else`)))
    (:`then_1`
      (bind _ascharacter (cast `Character` (`self.GetOwner`)))
      (bind _charactermovement (`Character.CharacterMovement` _ascharacter))
      (set `CharacterMovementComponent.GroundFriction` 1.0 _charactermovement)
      (set `CharacterMovementComponent.GravityScale` 1.0 _charactermovement)
      (set `CharacterMovementComponent.AirControl` 1.0 _charactermovement))))

(fn `OnGrappleHit`
  (params (SelfActor :type "Actor Object Reference") (OtherActor :type "Actor Object Reference") (NormalImpulse :type "Vector Structure") (Hit :type "HitResult Structure (by ref)"))
  (set `self.GrappleState` "NewEnumerator2")
  (bind _ascharacter (cast `Character` (`self.GetOwner`)))
  (bind _charactermovement (`Character.CharacterMovement` _ascharacter))
  (set `CharacterMovementComponent.GroundFriction` 0.0 _charactermovement)
  (set `CharacterMovementComponent.GravityScale` 0.06 _charactermovement)
  (set `CharacterMovementComponent.AirControl` 1.0 _charactermovement)
  (set `MovementComponent.Velocity` (+ (`MovementComponent.Velocity` _charactermovement) (* (`self.ToGrappleHook`) 1200.0)) _charactermovement)
  (set `self.InitialDirection2D` (`self.ToGrappleHook2D`)))